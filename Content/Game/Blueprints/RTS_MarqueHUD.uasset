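; RTS HUD that provides drag-box selection of units and exposes the resulting selection through GrabSelectedUnits.
; Marquee press, hold and release events track the mouse start and current positions and toggle drawing.
; While dragging, DrawHUD draws a translucent rectangle and queries Parent_Unit1 actors inside it every frame.
; It selects those units, clears the player controller's selected build, and deselects units outside the box, removing them while iterating the list.
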(event EventMarquePressed
  (bind _returnvalue (Game|GetPlayerController 0))
  (bind (_locationx _locationy) (Game|Player|GetMousePosition _returnvalue))
  (Variables|Default|SetIsDrawing? true)
  (bind _output_get (Variables|Default|SetStartMousePos (Math|Vector2D|MakeVector2D _locationx _locationy)))
  (Variables|Default|SetCurrentMousePos _output_get))

(event EventMarqueHeld
  (bind _returnvalue (Game|GetPlayerController 0))
  (bind (_locationx _locationy) (Game|Player|GetMousePosition _returnvalue))
  (Variables|Default|SetCurrentMousePos (Math|Vector2D|MakeVector2D _locationx _locationy)))

(event EventMarqueReleased
  (Variables|Default|SetIsDrawing? false))

(event EventDrawHUD
  (params (SizeX :type Integer) (SizeY :type Integer))
  (bind _startmousepos (Variables|Default|GetStartMousePos))
  (bind _currentmousepos (Variables|Default|GetCurrentMousePos))
  (bind _startmousepos_2 (Variables|Default|GetStartMousePos))
  (bind _currentmousepos_2 (Variables|Default|GetCurrentMousePos))
  (bind _outactors (Class|HUD|GetActorsinSelectionRectangle "/Game/Game/Blueprints/Parent_Unit1_Class.Parent_Unit1_Class_C" _startmousepos_2 _currentmousepos_2 false false))
  (if (Variables|Default|GetIsDrawing?)
    (HUD|DrawRect "(R=0.000000,G=0.026569,B=1.000000,A=0.200000)" (.x _startmousepos) (.y _startmousepos) (- (.x _currentmousepos) (.x _startmousepos)) (- (.y _currentmousepos) (.y _startmousepos)))
    (Variables|Default|SetActorInRectangle _outactors)
    (for _array_element _outactors
      (Class|RTSInterface|SelectThis(Message) _array_element)
      (Utilities|Array|AddUnique (Variables|Default|GetSelectedUnits) _array_element)
      (Class|RTSInterface|ClearSelectedBuild(Message) (Game|GetPlayerController 0)))
    (for _array_element_2 (Variables|Default|GetSelectedUnits)
      (if (== (Utilities|Array|FindItem (Variables|Default|GetActorInRectangle) _array_element_2) -1)
        (Class|RTSInterface|DeselectThis(Message) _array_element_2)
        (Utilities|Array|RemoveItem (Variables|Default|GetSelectedUnits) _array_element_2)))))

(fn ConstructionScript)

(fn GrabSelectedUnits
  (return (Variables|Default|GetSelectedUnits)))