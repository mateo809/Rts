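; Base building class for an RTS-style game that can be selected and produces AI units from a queue.
; On BeginPlay it creates its selection widget and fills the action box with its buttons; selecting toggles that widget and a decal.
; An authority-only looping timer takes queued units, tracks progress against each class's default production time, and spawns finished units at the Box location.
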(event Custom|AddUnitToQueue
  (params (Unit :type Parent%20Unit%201%20Class%20Class%20Reference))
  (Utilities|Array|Add (Variables|Default|GetUnitProductionQueue) Unit))

(event Custom|ProcessProductionunit
  (if (Variables|Default|GetIsProducingUnit?)
    (bind _output_get (Variables|Default|SetProductionTimeSpent (+ (Variables|Default|GetProductionTimeSpent) (Variables|Default|GetTime))))
    (bind _output_get_2 (Variables|Default|SetProductionProgress (/ _output_get (Variables|Default|GetProductionTimeNeeded))))
    (if (>= _output_get_2 1.0)
      (AI|SpawnAIFromClass (Variables|Default|GetUnitBeingProduced) 0 (Transformation|GetWorldLocation (Variables|Default|GetBox)) "0, 0, 0" false 0)
      (Variables|Default|SetProductionProgress 0.0)
      (Variables|Default|SetProductionTimeSpent 0.0)
      (Variables|Default|SetUnitBeingProduced 0)
      (Variables|Default|SetIsProducingUnit? false))
    (elif (> (Utilities|Array|Length (Variables|Default|GetUnitProductionQueue)) 0)
      (bind _output_get_3 (Variables|Default|SetUnitBeingProduced (Utilities|Array|Get(acopy) (Variables|Default|GetUnitProductionQueue))))
      (Variables|Default|SetProductionTimeNeeded (.ProductionTime (Utilities|GetClassDefaults _output_get_3)))
      (Utilities|Array|RemoveIndex (Variables|Default|GetUnitProductionQueue))
      (Variables|Default|SetIsProducingUnit? true))))

(event Collision|EventActorBeginOverlap
  (params (OtherActor :type Actor%20Object%20Reference)))

(event EventTick
  (params (DeltaSeconds :type Float%20%28single-precision%29)))

(event EventSelectThis
  (Rendering|SetVisibility (Variables|Default|GetDecal) true false)
  (UserInterface|Viewport|AddtoViewport (Variables|Default|GetBuildingSelectedVariable) 0))

(event EventDeselectThis
  (Rendering|SetVisibility (Variables|Default|GetDecal) false false)
  (Widget|RemovefromParent (Variables|Default|GetBuildingSelectedVariable)))

(event EventBeginPlay
  (Utilities|FlowControl|Sequence
    (:then_0
      (bind _returnvalue (UserInterface|CreateWidget "/Game/Game/Blueprints/Buildings/BuildingSelect.BuildingSelect_C"))
      (Variables|Default|SetBuildingSelectedVariable _returnvalue)
      (Variables|/Game/Game/Blueprints/Buildings/BuildingSelect.BuildingSelect_C|SetBuildingReference _returnvalue self)
      (for _array_element (Variables|Default|GetActionBoxButton)
        (Class|WrapBox|AddChildtoWrapBox (Variables|/Game/Game/Blueprints/Buildings/BuildingSelect.BuildingSelect_C|GetActionBox (Variables|Default|GetBuildingSelectedVariable)) _array_element)))
    (:then_1
      (Networking|SwitchHasAuthority
        (:Authority
          (Utilities|Time|SetTimerbyEvent (delegate Custom|ProcessProductionunit) (Variables|Default|GetTime) true))))))

(fn ConstructionScript)

(fn GrabSelectedUnits
  (return 0))

(fn ProduceUnit
  (params (Building :type Parent%20Building%20Class%20Object%20Reference) (Unit :type Parent%20Unit%201%20Class%20Class%20Reference)))