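; Iabuild is a child building Blueprint that offers a unit-production button for its action box.
; On BeginPlay it creates a Produce_Unit_2 widget, adds it to the ActionBoxButton array and sets itself as the widget's BuildingReference, then runs the parent BeginPlay.
; A matching Produce_Unit_1 setup is present but disconnected, and the construction script only calls its parent.
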(event EventBeginPlay
  (Utilities|FlowControl|Sequence
    (:then_1
      (bind _returnvalue (UserInterface|CreateWidget "/Game/Game/Blueprints/Buildings/Produce_Unit_2.Produce_Unit_2_C"))
      (Utilities|Array|AddUnique (Variables|Default|GetActionBoxButton) _returnvalue)
      (Variables|/Game/Game/Blueprints/Buildings/Produce_Unit_2.Produce_Unit_2_C|SetBuildingReference _returnvalue self))
    (:then_2
      (|CallParentFunction))))

(fn ConstructionScript
  (|CallParentFunction))