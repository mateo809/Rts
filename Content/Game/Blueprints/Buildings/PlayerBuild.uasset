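; PlayerBuild is a building Blueprint that supplies two unit-production buttons for an action box.
; On BeginPlay it creates Produce_Unit_1 and Produce_Unit_2 widgets, adds each to the ActionBoxButton array and sets itself as each one's BuildingReference.
; It calls the parent BeginPlay only after both buttons are registered, and its construction script just defers to the parent.
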(event EventBeginPlay
  (Utilities|FlowControl|Sequence
    (:then_0
      (bind _returnvalue (UserInterface|CreateWidget "/Game/Game/Blueprints/Buildings/Produce_Unit_1.Produce_Unit_1_C"))
      (Utilities|Array|AddUnique (Variables|Default|GetActionBoxButton) _returnvalue)
      (Variables|/Game/Game/Blueprints/Buildings/Produce_Unit_1.Produce_Unit_1_C|SetBuildingReference _returnvalue self))
    (:then_1
      (bind _returnvalue_2 (UserInterface|CreateWidget "/Game/Game/Blueprints/Buildings/Produce_Unit_2.Produce_Unit_2_C"))
      (Utilities|Array|AddUnique (Variables|Default|GetActionBoxButton) _returnvalue_2)
      (Variables|/Game/Game/Blueprints/Buildings/Produce_Unit_2.Produce_Unit_2_C|SetBuildingReference _returnvalue_2 self))
    (:then_2
      (|CallParentFunction))))

(fn ConstructionScript
  (|CallParentFunction))