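; Capture-point flag building that fills a capture percentage while a player unit or AI enemy stands in its sphere.
; Overlap matches only the first actor found of each class, then toggles decals and enables per-Tick, frame-rate-dependent progress.
; Any end overlap, or a non-matching begin overlap, resets progress.
; At full capture, Win only prints a placeholder string based on whether the overlapping actor is that unit.
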(event OnComponentBeginOverlap(Sphere)
  (params (OverlappedComponent :type Primitive%20Component%20Object%20Reference) (OtherActor :type Actor%20Object%20Reference) (OtherComp :type Primitive%20Component%20Object%20Reference) (OtherBodyIndex :type Integer) (bFromSweep :type Boolean) (SweepResult :type Hit%20Result%20Structure%20%28by%20ref%29))
  (bind _returnvalue (Actor|GetActorOfClass "/Game/Game/Blueprints/Buildings/IaBuilding/Ia_Enemy.Ia_Enemy_C"))
  (bind _returnvalue_2 (Actor|GetActorOfClass "/Game/Game/Blueprints/Parent_Unit1_Class.Parent_Unit1_Class_C"))
  (if (or (== OtherActor _returnvalue_2) (== OtherActor _returnvalue))
    (Variables|Default|SetIsEnter true)
    (Rendering|SetVisibility (Variables|Default|GetDecal) true false)
    (else
      (Variables|Default|SetCapturePourcent 0.0))))

(event OnComponentEndOverlap(Sphere)
  (params (OverlappedComponent :type Primitive%20Component%20Object%20Reference) (OtherActor :type Actor%20Object%20Reference) (OtherComp :type Primitive%20Component%20Object%20Reference) (OtherBodyIndex :type Integer))
  (Variables|Default|SetIsEnter false)
  (Variables|Default|SetCapturePourcent 0.0)
  (Rendering|SetVisibility (Variables|Default|GetDecal) false false))

(event Custom|CapturePoint
  (Variables|Default|SetCapturePourcent (Math|Float|Clamp(Float) (+ (Variables|Default|GetCapturePourcent) 0.05) 0.0 1e+02))
  (if (>= (Variables|Default|GetCapturePourcent) 1e+02)
    (CallFunction|Win)))

(event Custom|Win
  (bind _returnvalue (Actor|GetActorOfClass "/Game/Game/Blueprints/Parent_Unit1_Class.Parent_Unit1_Class_C"))
  (if (== (stale OnComponentBeginOverlap(Sphere) OtherActor) _returnvalue)
    (Development|PrintString "Meow")
    (else
      (Development|PrintString "Woaf"))))

(event EventTick
  (params (DeltaSeconds :type Float%20%28single-precision%29))
  (Rendering|SetVisibility (Variables|Default|GetDecal1) true false)
  (if (Variables|Default|GetIsEnter)
    (Rendering|SetVisibility (Variables|Default|GetDecal1) false false)
    (CallFunction|CapturePoint)
    (Development|PrintString (Utilities|String|ToString(Float) (Variables|Default|GetCapturePourcent)))))

(fn ConstructionScript)