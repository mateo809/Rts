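; RessourceCollector is a worker unit that shuttles between a resource node and a drop-off building to gather resources.
; SetIsWorking stores the node, looks for the nearest building by distance and starts the trip.
; Collect runs a timed mining phase with particle effects, then the unit carries its load to the building.
; Dropoff credits the first player controller and sends the unit back, while SetNotWorking halts the loop.
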(event Custom|RessourceCollected
  (Utilities|Time|ClearandInvalidateTimerbyHandle (Variables|Default|GetRessourceCollectTimer))
  (Variables|Default|SetHasRessource? true)
  (CallFunction|UnitMoveCommand (Transformation|GetActorLocation (Variables|Default|GetDropoffBuilding)))
  (Components|Activation|SetActive (Variables|Default|GetParticleSystem) false false))

(event Custom|ActiveSFXMining
  (Components|Activation|SetActive (Variables|Default|GetParticleSystem) true false))

(event EventDropoff
  (if (Variables|Default|GetIsWorking)
    (if (Variables|Default|GetHasRessource?)
      (Class|RTSInterface|IncrementeRessource(Message) (Game|GetPlayerController 0) 10)
      (Variables|Default|SetHasRessource? false)
      (CallFunction|UnitMoveCommand (Transformation|GetActorLocation (Variables|Default|GetRessourceNode)))
      (else
        (CallFunction|UnitMoveCommand (Transformation|GetActorLocation (Variables|Default|GetRessourceNode)))))))

(event EventSetNotWorking
  (Variables|Default|SetIsWorking false)
  (Utilities|Time|ClearandInvalidateTimerbyHandle (Variables|Default|GetRessourceCollectTimer)))

(event EventCollect
  (if (Variables|Default|GetIsWorking)
    (if (Variables|Default|GetHasRessource?)
      (CallFunction|UnitMoveCommand (Transformation|GetActorLocation (Variables|Default|GetDropoffBuilding)))
      (elif (not (Utilities|Time|IsValidTimerHandle (Variables|Default|GetRessourceCollectTimer)))
        (CallFunction|ActiveSFXMining)
        (CallFunction|UnitMoveCommand (Transformation|GetActorLocation))
        (bind _returnvalue (Utilities|Time|SetTimerbyEvent (delegate Custom|RessourceCollected) 4.0))
        (Variables|Default|SetRessourceCollectTimer _returnvalue)))))

(event EventSetIsWorking
  (params (RessourceNode :type Actor%20Object%20Reference))
  (Variables|Default|SetIsWorking true)
  (Variables|Default|SetRessourceNode RessourceNode)
  (bind _outactors (Actor|GetAllActorsOfClass "/Game/Game/Blueprints/Buildings/Parent_Building_Class.Parent_Building_Class_C"))
  (for _array_element _outactors
    (if (< (Transformation|GetDistanceTo _array_element self) (Variables|Default|GetClosetDropOffBuildingDistance))
      (Variables|Default|SetDropoffBuilding _array_element)
      (Variables|Default|SetClosetDropOffBuildingDistance (Transformation|GetDistanceTo _array_element self))))
  (if (Variables|Default|GetHasRessource?)
    (CallFunction|UnitMoveCommand (Transformation|GetActorLocation (Variables|Default|GetDropoffBuilding)))
    (else
      (CallFunction|UnitMoveCommand (Transformation|GetActorLocation (Variables|Default|GetRessourceNode))))))

(fn ConstructionScript
  (|CallParentFunction))