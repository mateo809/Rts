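; Player-side combat unit, apparently a character, that shoots at Ia_Enemy actors inside its Sphere and is destroyed when health runs out.
; Tick loops over overlapping enemies, spawning Bp_Projectile at the Shoot transform behind a Cooldown delay.
; Sphere overlap with the first Ia_Enemy found sets Attack, halts movement and turns the unit toward it once.
; Hovering the mesh shows the Radius component, with mouse-over events enabled from Tick.
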(event OnComponentBeginOverlap(Sphere)
  (params (OverlappedComponent :type Primitive%20Component%20Object%20Reference) (OtherActor :type Actor%20Object%20Reference) (OtherComp :type Primitive%20Component%20Object%20Reference) (OtherBodyIndex :type Integer) (bFromSweep :type Boolean) (SweepResult :type Hit%20Result%20Structure%20%28by%20ref%29))
  (bind _returnvalue (Actor|GetActorOfClass "/Game/Game/Blueprints/Buildings/IaBuilding/Ia_Enemy.Ia_Enemy_C"))
  (if (== OtherActor _returnvalue)
    (Variables|Default|SetAttack? true)
    (Components|Movement|StopMovementImmediately (Variables|Character|GetCharacterMovement))
    (Transformation|SetActorRotation self (Math|Rotator|FindLookatRotation (Transformation|GetActorLocation) (Transformation|GetActorLocation OtherActor)))))

(event OnEndCursorOver(StaticMesh)
  (params (TouchedComponent :type Primitive%20Component%20Object%20Reference))
  (Rendering|SetVisibility (Variables|Default|GetRadius) false false))

(event OnBeginCursorOver(StaticMesh)
  (params (TouchedComponent :type Primitive%20Component%20Object%20Reference))
  (Rendering|SetVisibility (Variables|Default|GetRadius) true false))

(event Collision|EventActorBeginOverlap
  (params (OtherActor :type Actor%20Object%20Reference))
  (|CallParentFunction OtherActor) ; Ce nœud est désactivé et ne sera pas appelé.\nFaites glisser les broches pour générer des fonctionnalités.
)

(event EventTick
  (params (DeltaSeconds :type Float%20%28single-precision%29))
  (if (<= (Variables|Default|GetCurrentHealth) 0)
    (Actor|DestroyActor self)
    (else
      (Variables|/Script/Engine.PlayerController|SetbEnableMouseOverEvents (Game|GetPlayerController 0) true)
      (Utilities|Array|ForEachLoopwithBreak (Collision|GetOverlappingActors (Variables|Default|GetSphere) "/Game/Game/Blueprints/Buildings/IaBuilding/Ia_Enemy.Ia_Enemy_C" :!class /Script/Engine.PrimitiveComponent)
        (:LoopBody
          (Utilities|FlowControl|Delay (Variables|Default|GetCooldown))
          (Game|SpawnActorfromClass "/Game/Game/Blueprints/Bp_Projectile.Bp_Projectile_C" (Transformation|GetWorldTransform (Variables|Default|GetShoot)) "AlwaysSpawn" "MultiplyWithRoot" 0 0))))))

(fn ConstructionScript
  (|CallParentFunction))